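; BP_Cube_video is an actor that opens a concept video on a media player at BeginPlay and gives its cube a dynamic material instance.
; StartFadeOut prints a completion message, plays a fade timeline and destroys the actor when it finishes.
; The end-of-video binding and the material Fade update are disconnected, so nothing in this graph triggers the fade-out or changes the material's opacity parameter.
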(event `self.ReceiveBeginPlay`
  (`MediaPlayer.OpenSource` (`self.Mediaplayer`) "/Game/Movies/CONCEPT_V2_INGEKORT.CONCEPT_V2_INGEKORT")
  (bind _returnvalue (`PrimitiveComponent.CreateDynamicMaterialInstance` (`self.Cube`) 0 "/Game/Movies/KOPIE_CONCEPT_V2_Materiaal1.KOPIE_CONCEPT_V2_Materiaal1" "None"))
  (set `self.NewVar` _returnvalue))

(event `StartFadeOut`
  (`KismetSystemLibrary.PrintString` "Video klaar!")
  (bind (_direction _fade) (`Timeline|FadeTimeLine`)
    (:`Finished`
      (`self.K2_DestroyActor`))))

(fn `UserConstructionScript`)